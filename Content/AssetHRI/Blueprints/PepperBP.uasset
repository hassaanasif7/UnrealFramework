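; Pawn Blueprint for a Pepper robot that shows the Pepper_W widget, moves via AI and speaks text aloud.
; MoveRobot issues AIMoveTo to a CalculateLocation destination, tracking IsMoving until success; BeginPlay also sends an initial move.
; SaySomething feeds a macro that plays Microsoft text-to-speech as 2D sound, then after a delay records audio output to a WAV in the project directory.
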(event EventMoveRobot
  (params (X :type Float%20%28single-precision%29) (Y :type Float%20%28single-precision%29))
  (Variables|Default|SetIs%20Moving? true)
  (AI|AIMoveTo self (Utilities|CalculateLocation X Y) 0 5.0 false
    (:OnSuccess
      (Variables|Default|SetIs%20Moving? false))))

(event EventBeginPlay
  (bind _returnvalue (UserInterface|CreateWidget "/Game/AssetHRI/Widgets/Pepper_W.Pepper_W_C"))
  (UserInterface|Viewport|AddtoViewport _returnvalue 0)
  (AI|AIMoveTo self (Utilities|CalculateLocation 2e+02 2e+02) 0 5.0 false))

(event EventSaySomething
  (params (Text :type String))
  (|Microphone&Speaker_2 Text))

(fn ConstructionScript)