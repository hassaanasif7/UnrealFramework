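; Blueprint for a controllable NAO robot that can move, speak and play posture animations, showing its NAO_W widget on begin play.
; MoveRobot uses AI MoveTo to a destination computed from an X/Y offset to its location, tracking IsMoving until success.
; SaySomething plays text-to-speech, then after a delay records audio output to a WAV in the project directory.
; Postures plays stand-to-rest, then rest-to-stand on a timed delay.
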(event OnComponentBeginOverlap(B2)
  (params (OverlappedComponent :type Primitive%20Component%20Object%20Reference) (OtherActor :type Actor%20Object%20Reference) (OtherComp :type Primitive%20Component%20Object%20Reference) (OtherBodyIndex :type Integer) (bFromSweep :type Boolean) (SweepResult :type Hit%20Result%20Structure%20%28by%20ref%29)))

(event Custom|Postures
  (bind _mesh (Variables|Character|GetMesh))
  (Variables|Default|SetIsMoving? false)
  (Components|Animation|PlayAnimation _mesh "/Game/AssetHRI/Animations/StandToRest_Anim.StandToRest_Anim" false)
  (Utilities|FlowControl|Delay 7.5)
  (Components|Animation|PlayAnimation _mesh "/Game/AssetHRI/Animations/RestStand.RestStand" false))

(event EventMoveRobot
  (params (X :type Float%20%28single-precision%29) (Y :type Float%20%28single-precision%29))
  (Variables|Default|SetIsMoving? true)
  (AI|AIMoveTo self (Utilities|CalculateLocation X Y) 0 5.0 false
    (:OnSuccess
      (Variables|Default|SetIsMoving? false))))

(event EventSaySomething
  (params (Text :type String))
  (|Microphone&Speaker Text))

(event EventBeginPlay
  (bind _returnvalue (UserInterface|CreateWidget "/Game/AssetHRI/Widgets/NAO_W.NAO_W_C"))
  (UserInterface|Viewport|AddtoViewport _returnvalue 0))

(fn ConstructionScript)